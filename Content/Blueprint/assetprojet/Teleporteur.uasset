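; Teleporter entrance that moves the player to a linked exit when the player character overlaps its sphere.
; It searches all Interupteur switches for one matching its Identre ID and continues only if that switch is activated.
; It then finds each Teleporteursortie whose IDsortie matches the same ID and sets the player's location to that exit's position.
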(event OnComponentBeginOverlap(Sphere)
  (params (OverlappedComponent :type Primitive%20Component%20Object%20Reference) (OtherActor :type Actor%20Object%20Reference) (OtherComp :type Primitive%20Component%20Object%20Reference) (OtherBodyIndex :type Integer) (bFromSweep :type Boolean) (SweepResult :type Hit%20Result%20Structure%20%28by%20ref%29))
  (bind _returnvalue (Game|GetPlayerCharacter 0))
  (if (== OtherActor _returnvalue)
    (bind _outactors (Actor|GetAllActorsOfClass "/Game/Blueprint/assetprojet/interupteur.interupteur_C"))
    (for _array_element _outactors
      (if (== (Variables|/Game/Blueprint/assetprojet/interupteur.interupteur_C|GetIDinterupteur _array_element) (Variables|Default|Getidentre))
        (if (Variables|/Game/Blueprint/assetprojet/interupteur.interupteur_C|GetActiver _array_element)
          (bind _outactors_2 (Actor|GetAllActorsOfClass "/Game/Blueprint/assetprojet/Teleporteursortie.Teleporteursortie_C"))
          (for _array_element_2 _outactors_2
            (if (== (Variables|/Game/Blueprint/assetprojet/Teleporteursortie.Teleporteursortie_C|GetIDsortie _array_element_2) (Variables|Default|Getidentre))
              (bind _output_get (Variables|Default|Setnouvelle%20position (Transformation|GetActorLocation _array_element_2)))
              (switch int 0
                (:0
                  (Transformation|SetActorLocation _returnvalue _output_get false false))
                (:1
                  (Transformation|SetActorLocation _returnvalue _output_get false false))))))))))

(fn ConstructionScript)