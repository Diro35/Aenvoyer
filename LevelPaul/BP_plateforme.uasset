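; BP_plateforme is a moving platform that travels from its starting position toward an EndPoint component when triggered by an overlap.
; BeginPlay caches the world locations of Platform and EndPoint.
; When Player_touch begins overlapping an actor that casts to PlayerStart, rather than a pawn or character, a timeline plays and lerps Platform between those locations without sweeping.
; No reverse movement is wired.
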(event OnComponentBeginOverlap(Player_touch)
  (params (OverlappedComponent :type Primitive%20Component%20Object%20Reference) (OtherActor :type Actor%20Object%20Reference) (OtherComp :type Primitive%20Component%20Object%20Reference) (OtherBodyIndex :type Integer) (bFromSweep :type Boolean) (SweepResult :type Hit%20Result%20Structure%20%28by%20ref%29))
  (Utilities|Casting|CastToPlayerStart OtherActor)
  (bind _newtrack_0 (Timeline|Timeline_0 Play)
    (:Update
      (Transformation|SetWorldLocation (Variables|Default|GetPlatform) (Math|Vector|Lerp(Vector) (Variables|Default|GetLocation_depart) (Variables|Default|GetLocation_end) _newtrack_0) false false))))

(event EventBeginPlay
  (Variables|Default|SetLocation_depart (Transformation|GetWorldLocation (Variables|Default|GetPlatform)))
  (Variables|Default|SetLocation_end (Transformation|GetWorldLocation (Variables|Default|GetEnd_point))))

(event Collision|EventActorBeginOverlap
  (params (OtherActor :type Actor%20Object%20Reference)))

(event EventTick
  (params (DeltaSeconds :type Float%20%28single-precision%29)))

(fn ConstructionScript)